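; BP_ScalableBattleMat is a battle mat actor that is sized and styled entirely in its construction script, with no active event logic.
; When either mat dimension exceeds one, it stretches the static mesh in X and Y by AdditiveScale per extra unit, added to its current world scale.
; It picks the material from MaterialMap by LandscapeType, then feeds MatSettings into a dynamic instance for base color, texture alpha and compass rose appearance.
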(fn `UserConstructionScript`
  (bind _staticmesh (`self.StaticMesh`))
  (bind _matdimention_y (`self.MatDimention_Y`))
  (bind _staticmesh_2 (`self.StaticMesh`))
  (bind _matdimention_x (`self.MatDimention_X`))
  (bind (_matbasecolor _mattexturealpha _roseofwindscolor _roseofwindsalpha _roseofwindsscale _roseofwindsposition) (break `/Game/DungeonsOfDice/Blueprints/BattleMat/Str_MatSettingsStructure` (`self.MatSettings`)))
  (bind (_returnvalue_x _returnvalue_y _returnvalue_z) (`KismetMathLibrary.BreakVector` (`SceneComponent.K2_GetComponentScale` _staticmesh)))
  (bind _returnvalue (* (- _matdimention_x 1) (`self.AdditiveScale`)))
  (bind (_x _y) (`KismetMathLibrary.BreakVector2D` _roseofwindsposition))
  (if (or (> _matdimention_x 1) (> _matdimention_y 1))
    (`SceneComponent.SetRelativeScale3D` _staticmesh (`KismetMathLibrary.MakeVector` (+ _returnvalue _returnvalue_x) (+ (select `bool` false :`false` (* (- _matdimention_y 1) (`self.AdditiveScale`)) :`true` _returnvalue) _returnvalue_y) _returnvalue_z)))
  (`PrimitiveComponent.SetMaterial` _staticmesh_2 0 (`BlueprintMapLibrary.Map_Find` (`self.MaterialMap`) (`self.LandscapeType`)))
  (bind _returnvalue_2 (`PrimitiveComponent.CreateDynamicMaterialInstance` _staticmesh_2 0 null "None"))
  (`MaterialInstanceDynamic.SetVectorParameterValue` _returnvalue_2 "MatBaseColor" _matbasecolor)
  (`MaterialInstanceDynamic.SetScalarParameterValue` _returnvalue_2 "TextureAlpha" _mattexturealpha)
  (`MaterialInstanceDynamic.SetVectorParameterValue` _returnvalue_2 "RoseColor" _roseofwindscolor)
  (`MaterialInstanceDynamic.SetScalarParameterValue` _returnvalue_2 "RoseAlpha" _roseofwindsalpha)
  (`MaterialInstanceDynamic.SetScalarParameterValue` _returnvalue_2 "RoseScale" _roseofwindsscale)
  (`MaterialInstanceDynamic.SetScalarParameterValue` _returnvalue_2 "RoseU_Position" _x)
  (`MaterialInstanceDynamic.SetScalarParameterValue` _returnvalue_2 "RoseV_Position" _y))