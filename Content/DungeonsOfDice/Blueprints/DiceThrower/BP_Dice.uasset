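; BP_Dice is a physical die actor that tumbles, comes to rest and reports its rolled value to BP_DiceTray.
; Construction picks the mesh by DiceType; a random per-tick spin runs until the first hit.
; Once velocity reaches zero, the highest mesh socket identifies the top face, which SocketToSideMap converts to a value.
; The mesh's socket count determines the die type sent with that result.
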(event `SetDiceValues`
  (bind _dice (`self.Dice`))
  (bind _dicetray (`self.DiceTray`))
  (bind _returnvalue (`SceneComponent.GetAllSocketNames` _dice))
  ;[1 1 1] Find Hiest Socket and Send Info
  (for _array_element _returnvalue
    (bind _z (.z (`SceneComponent.GetSocketLocation` _dice _array_element)))
    (if (not (< _z (`self.MinValue`)))
      (set `self.MinValue` _z)
      (bind _output_get (set `self.CurrentSocketName` _array_element))))
  (bind _output_get_2 (set `self.DiceValue` (`BlueprintMapLibrary.Map_Find` (`self.SocketToSideMap`) _output_get)))
  (`/Engine/EditorBlueprintResources/StandardMacros.IsValid` _dicetray
    (:`Is Valid`
      (message `/Game/DungeonsOfDice/Blueprints/DiceThrower/BPI_GetDiceValues.GetDiceValues` _dicetray _output_get_2 (`BlueprintMapLibrary.Map_Find` (`self.SidesToType`) (`KismetArrayLibrary.Array_Length` _returnvalue))))))

(event `self.ReceiveTick`
  (params (DeltaSeconds :type "Float (single-precision)"))
  ;[1 1 1] Rotate and Wait for Dice to Stop
  (`/Engine/EditorBlueprintResources/StandardMacros.Gate` true :!label _label
    (:`Exit`
      (if (`self.AddRotation?`)
        (`self.K2_AddActorWorldRotation` (`self.RandomRotation`)))
      (if (== (`self.GetVelocity`) (0.0 0.0 0.0))
        (`|ExecutionSequence`
          (:`then_0`
            (`/Engine/EditorBlueprintResources/StandardMacros.DoOnce` false
              (:`Completed`
                (`self.SetDiceValues`))))
          (:`then_1`
            (goto _label :!via `Close`)))))))

(event `self.ReceiveBeginPlay`
  ;[1 1 1] Initial Spawn
  (bind _outactors (`GameplayStatics.GetAllActorsOfClass` "/Game/DungeonsOfDice/Blueprints/DiceThrower/BP_DiceTray.BP_DiceTray_C"))
  (set `self.DiceTray` (`|GetArrayItem` _outactors))
  (set `self.DiceType` (`BlueprintMapLibrary.Map_Find` (`self.SidesToType`) (`KismetArrayLibrary.Array_Length` (`SceneComponent.GetAllSocketNames` (`self.Dice`)))))
  (set `self.RandomRotation` (`KismetMathLibrary.MakeRotator` (`KismetMathLibrary.RandomFloatInRange` 0.0 5.0) (`KismetMathLibrary.RandomFloatInRange` 0.0 5.0) (`KismetMathLibrary.RandomFloatInRange` 0.0 5.0)))
  (goto _label :!via `Open`))

(event `self.Dice.OnComponentHit`
  (params (HitComponent :type "PrimitiveComponent Object Reference") (OtherActor :type "Actor Object Reference") (OtherComp :type "PrimitiveComponent Object Reference") (NormalImpulse :type "Vector Structure") (Hit :type "HitResult Structure (by ref)"))
  ;[1 1 1] Stop Dice Rotation on Hit
  (if (`self.AddRotation?`)
    (set `self.AddRotation?` false)))

(fn `UserConstructionScript`
  (`StaticMeshComponent.SetStaticMesh` (`self.Dice`) (`|GetArrayItem` (`self.DiceMeshes`) (`self.DiceType`))))