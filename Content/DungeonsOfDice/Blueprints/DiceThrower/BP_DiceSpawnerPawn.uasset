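; BP_DiceSpawnerPawn is a pawn that throws dice into the Dungeons of Dice scene and shows the mouse cursor on begin play.
; Its SpawnDice event spawns a half-scale BP_Dice of the requested DiceType just below the pawn.
; Each die gets a randomized pitch and yaw around a fixed facing, then is added to the SpawnedDice array.
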(event `self.ReceiveBeginPlay`
  (set `PlayerController.bShowMouseCursor` true (`GameplayStatics.GetPlayerController` 0)))

(event `SpawnDice`
  (params (DiceType :type Integer))
  (bind _returnvalue (`|SpawnActorFromClass` "/Game/DungeonsOfDice/Blueprints/DiceThrower/BP_Dice.BP_Dice_C" (`KismetMathLibrary.MakeTransform` (`KismetMathLibrary.MakeVector` (.x (`self.K2_GetActorLocation`)) (.y (`self.K2_GetActorLocation`)) (- (.z (`self.K2_GetActorLocation`)) 200.0)) (`KismetMathLibrary.MakeRotator` 0.0 (`KismetMathLibrary.RandomFloatInRange` -65.0 10.0) (+ -90.0 (`KismetMathLibrary.RandomFloatInRange` -25.0 25.0))) (0.5 0.5 0.5)) "Undefined" "OverrideRootScale" null DiceType null))
  (`KismetArrayLibrary.Array_Add` (`self.SpawnedDice`) _returnvalue))

(fn `UserConstructionScript`)