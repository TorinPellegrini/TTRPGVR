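; Enemy actor for a tabletop RPG game, with a selection marker and a skeletal mesh animated through events.
; A cone starts hidden and is shown or hidden by the select and deselect events.
; Animation events play clips directly on the mesh without an Anim Blueprint state machine; attack and taunt return to looping idle after hardcoded delays, while death plays once.
; Tick is empty, with its interval lengthened at BeginPlay.
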(event `self.ReceiveBeginPlay`
  (`SceneComponent.SetVisibility` (`self.Cone`) false false)
  (`self.SetActorTickInterval` 0.5))

(event `self.ReceiveTick`
  (params (DeltaSeconds :type "Float (single-precision)")))

(event `SelectEnemy`
  (`SceneComponent.SetVisibility` (`self.Cone`) true false))

(event `DeselectEnemy`
  (`SceneComponent.SetVisibility` (`self.Cone`) false false))

(event `PlayAttackAnim`
  (bind _skeletalmesh (`self.SkeletalMesh`))
  (`SkeletalMeshComponent.PlayAnimation` _skeletalmesh "/Game/TTRPG/GameObjects/Enemy/GoblinAssets/Zombie_Attack_Anim_mixamo_com.Zombie_Attack_Anim_mixamo_com" false)
  (`KismetSystemLibrary.Delay` 2.75)
  (`SkeletalMeshComponent.PlayAnimation` _skeletalmesh "/Game/TTRPG/GameObjects/Enemy/GoblinAssets/Zombie_Idle_Anim_mixamo_com.Zombie_Idle_Anim_mixamo_com" true))

(event `PlayTauntAnim`
  (bind _skeletalmesh (`self.SkeletalMesh`))
  (`SkeletalMeshComponent.PlayAnimation` _skeletalmesh "/Game/TTRPG/GameObjects/Enemy/GoblinAssets/Loser_Anim_mixamo_com.Loser_Anim_mixamo_com" false)
  (`KismetSystemLibrary.Delay` 3.3)
  (`SkeletalMeshComponent.PlayAnimation` _skeletalmesh "/Game/TTRPG/GameObjects/Enemy/GoblinAssets/Zombie_Idle_Anim_mixamo_com.Zombie_Idle_Anim_mixamo_com" true))

(event `PlayDeathAnim`
  (`SkeletalMeshComponent.PlayAnimation` (`self.SkeletalMesh`) "/Game/TTRPG/GameObjects/Enemy/GoblinAssets/Sword_And_Shield_Death_Anim_mixamo_com.Sword_And_Shield_Death_Anim_mixamo_com" false))

(event `PlayIdleAnim`
  (`SkeletalMeshComponent.PlayAnimation` (`self.SkeletalMesh`) "/Game/TTRPG/GameObjects/Enemy/GoblinAssets/Zombie_Idle_Anim_mixamo_com.Zombie_Idle_Anim_mixamo_com" true))

(fn `UserConstructionScript`)