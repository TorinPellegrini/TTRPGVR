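; BP_Dice is a grippable physics die for a tabletop RPG, thrown with the releasing controller's velocity as an impulse.
; After release, Tick waits for it to stop, then maps the highest mesh socket to a face value.
; The result plus modifier is broadcast and shown to the player before the die expires.
; Socket count determines DiceType, whose OnRep swaps the mesh; arrow-based DetermineSide is uncalled here.
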(event `SetDiceValues`
  (bind _dicemesh (`self.DiceMesh`))
  ;[1 1 1] Find Dice Values from socket
  (for _array_element (`SceneComponent.GetAllSocketNames` _dicemesh)
    (bind _z (.z (`SceneComponent.GetSocketLocation` _dicemesh _array_element)))
    (if (not (< _z (`self.MinValue`)))
      (set `self.MinValue` _z)
      (bind _output_get (set `self.CurrentSocketName` _array_element))))
  (bind _output_get_2 (set `self.DiceValue` (`BlueprintMapLibrary.Map_Find` (`self.SocketToSideMap`) _output_get)))
  (bind _returnvalue (+ _output_get_2 (`self.RollModifier`)))
  ;[1 1 1] Broadcast Result
  (`self.RollResult` _returnvalue)
  (`self.SetLifeSpan` 5.0)
  ;[1 1 1] Display Dice Results
  (bind _output_get_3 (set `self.DiceRollString` "Die rolled a "))
  (bind _ascharacter_default (cast `/Game/TTRPG/Character/Character_Default` (`Controller.K2_GetPawn` (`GameplayStatics.GetPlayerController` 0)))
    (:`then`
      (`/Game/TTRPG/Character/Character_Default.DisplayNotification` _ascharacter_default (`KismetStringLibrary.Concat_StrStr` _output_get_3 (`KismetStringLibrary.Conv_IntToString` _returnvalue))))
    (:`CastFailed`
      (`KismetSystemLibrary.PrintString` "Cast to player fail"))))

(event `self.ReceiveBeginPlay`
  ;[1 1 1] Set Rotator and get Dice on BeginPlay
  (set `self.Sides` (`self.K2_GetComponentsByClass` "/Script/Engine.ArrowComponent"))
  (set `self.DiceType` (`BlueprintMapLibrary.Map_Find` (`self.SidesToType`) (`KismetArrayLibrary.Array_Length` (`SceneComponent.GetAllSocketNames` (`self.DiceMesh`)))))
  (set `self.RandomRotation` (`KismetMathLibrary.MakeRotator` (`KismetMathLibrary.RandomFloatInRange` 0.0 5.0) (`KismetMathLibrary.RandomFloatInRange` 0.0 5.0) (`KismetMathLibrary.RandomFloatInRange` 0.0 5.0)))
  (`self.SetActorTickEnabled` false))

(event `self.ReceiveTick`
  (params (DeltaSeconds :type "Float (single-precision)"))
  ;[1 1 1] Roll Dice on Tick
  (if (== (`SceneComponent.GetComponentVelocity` (`self.DiceMesh`)) (0.0 0.0 0.0))
    (`self.SetDiceValues`)
    (`self.SetActorTickEnabled` false)))

(event `VRGripInterface.OnGripRelease`
  (params (ReleasingController :type "GripMotionControllerComponent Object Reference") (GripInformation :type "BPActorGripInformation Structure (by ref)") (bWasSocketed :type Boolean))
  (bind _dicemesh (`self.DiceMesh`))
  ;[1 1 1] Roll when thrown
  (`PrimitiveComponent.SetSimulatePhysics` _dicemesh true)
  (`PrimitiveComponent.AddImpulse` _dicemesh (* (`SceneComponent.GetComponentVelocity` ReleasingController) 10.0) "None" false)
  (`KismetSystemLibrary.Delay` 0.2)
  (`self.SetActorTickEnabled` true))

(fn `DetermineSide`
  (params (Array :type "Array of ArrowComponent Object Reference"))
  (returns (DiceRollResult :type String))
  (bind _returnvalue (`KismetSystemLibrary.GetObjectName` (`self.ClosestUp`)))
  (set `self.Dot` -10000.0)
  (set `self.ClosestUp` null)
  (for _array_element Array
    (bind _returnvalue_2 (`KismetMathLibrary.Dot_VectorVector` (`SceneComponent.GetForwardVector` _array_element) (0.0 0.0 1.0)))
    (if (> _returnvalue_2 (`self.Dot`))
      (set `self.Dot` _returnvalue_2)
      (set `self.ClosestUp` _array_element)))
  (`KismetSystemLibrary.PrintString` _returnvalue)
  (bind _output_get (set `self.DiceRollString` "Die rolled a "))
  (return (`KismetStringLibrary.Concat_StrStr` _output_get _returnvalue)))

(fn `OnRep_DiceType`
  (`StaticMeshComponent.SetStaticMesh` (`self.DiceMesh`) (`|GetArrayItem` (`self.DiceMeshes`) (`self.DiceType`))))

(fn `UserConstructionScript`)