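; Throwable tabletop die, likely eight-sided, that reports which side lands up after a roll.
; On grip release it simulates physics, applies torque and impulse from the controller's velocity, then arms the rest check after a short delay.
; Tick waits for near-zero velocity, then once per throw picks the Arrow component pointing most upward by dot product.
; That component's name becomes the result notification on the player's Character_Default pawn.
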(event `self.ReceiveTick`
  (params (DeltaSeconds :type "Float (single-precision)"))
  (if (and (<= (`KismetMathLibrary.VSize` (`self.GetVelocity`)) 1.0) (`self.CheckForDiceRoll`))
    (`/Engine/EditorBlueprintResources/StandardMacros.DoOnce` false :!label _label
      (:`Completed`
        (`PrimitiveComponent.SetAllPhysicsLinearVelocity` (`self.DiceMesh`) (0.0 0.0 0.0) false)
        (bind _dicerollresult (`self.DetermineSide` (`self.Sides`)))
        (bind _ascharacter_default (cast `/Game/TTRPG/Character/Character_Default` (`Controller.K2_GetPawn` (`GameplayStatics.GetPlayerController` 0)))
          (:`then`
            (`/Game/TTRPG/Character/Character_Default.DisplayNotification` _ascharacter_default _dicerollresult))
          (:`CastFailed`
            (`KismetSystemLibrary.PrintString` "Cast to player fail")))))))

(event `VRGripInterface.OnGripRelease`
  (params (ReleasingController :type "GripMotionControllerComponent Object Reference") (GripInformation :type "BPActorGripInformation Structure (by ref)") (bWasSocketed :type Boolean))
  (bind _outlinearvelocity (`MotionControllerComponent.GetLinearVelocity` ReleasingController))
  (bind _dicemesh (`self.DiceMesh`))
  (`|ExecutionSequence`
    (:`then_0`
      (goto _label :!via `Reset`))
    (:`then_1`
      (`PrimitiveComponent.SetSimulatePhysics` _dicemesh true)
      (`PrimitiveComponent.AddTorqueInRadians` _dicemesh (* _outlinearvelocity 2.0) "None" true)
      (`PrimitiveComponent.AddImpulse` _dicemesh (* _outlinearvelocity 10.0) "None" false)
      (set `self.CheckForDiceRoll` false)
      (`KismetSystemLibrary.Delay` 0.3)
      (set `self.CheckForDiceRoll` true))))

(event `self.ReceiveBeginPlay`
  (set `self.Sides` (`self.K2_GetComponentsByClass` "/Script/Engine.ArrowComponent")))

(fn `DetermineSide`
  (params (Array :type "Array of ArrowComponent Object Reference"))
  (returns (DiceRollResult :type String))
  (bind _returnvalue (`KismetSystemLibrary.GetObjectName` (`self.ClosestUp`)))
  (set `self.Dot` -10000.0)
  (set `self.ClosestUp` null)
  (for _array_element Array
    (bind _returnvalue_2 (`KismetMathLibrary.Dot_VectorVector` (`SceneComponent.GetForwardVector` _array_element) (0.0 0.0 1.0)))
    (if (> _returnvalue_2 (`self.Dot`))
      (set `self.Dot` _returnvalue_2)
      (set `self.ClosestUp` _array_element)))
  (`KismetSystemLibrary.PrintString` _returnvalue)
  (bind _output_get (set `self.DiceRollString` "Die rolled a "))
  (return (`KismetStringLibrary.Concat_StrStr` _output_get _returnvalue)))

(fn `UserConstructionScript`)