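; BP_SixDice is a physics-driven six-sided die that detects which face lands up.
; On BeginPlay and grip release, it enables physics on the cube and gives it a random rotation.
; Once velocity first drops near zero, a DoOnce, never reset, stops the cube and runs DetermineSide.
; That function picks the arrow component whose forward vector best matches world up and prints its name.
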(event `self.ReceiveTick`
  (params (DeltaSeconds :type "Float (single-precision)"))
  (if (<= (`KismetMathLibrary.VSize` (`self.GetVelocity`)) 1.0)
    (`/Engine/EditorBlueprintResources/StandardMacros.DoOnce` false
      (:`Completed`
        (`PrimitiveComponent.SetAllPhysicsLinearVelocity` (`self.Cube`) (0.0 0.0 0.0) false)
        (`self.DetermineSide` (`self.Sides`))))))

(event `VRGripInterface.OnGripRelease`
  (params (ReleasingController :type "GripMotionControllerComponent Object Reference") (GripInformation :type "BPActorGripInformation Structure (by ref)") (bWasSocketed :type Boolean))
  (bind _cube (`self.Cube`))
  (`PrimitiveComponent.SetSimulatePhysics` _cube true :!label _label)
  (`SceneComponent.K2_SetWorldRotation` _cube (`KismetMathLibrary.RandomRotator` false) false false))

(event `self.ReceiveBeginPlay`
  (set `self.Sides` (`self.K2_GetComponentsByClass` "/Script/Engine.ArrowComponent"))
  (goto _label))

(fn `DetermineSide`
  (params (Array :type "Array of ArrowComponent Object Reference"))
  (set `self.Dot` -10000.0)
  (set `self.ClosestUp` null)
  (for _array_element Array
    (bind _returnvalue (`KismetMathLibrary.Dot_VectorVector` (`SceneComponent.GetForwardVector` _array_element) (0.0 0.0 1.0)))
    (if (> _returnvalue (`self.Dot`))
      (set `self.Dot` _returnvalue)
      (set `self.ClosestUp` _array_element)))
  (`KismetSystemLibrary.PrintString` (`KismetSystemLibrary.GetDisplayName` (`self.ClosestUp`))))

(fn `UserConstructionScript`)