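; Game mode for a VR tabletop RPG that sets up joining players and relays session events.
; On login it spawns a default character at the world origin, possesses it and tracks it in a pawn list, from which DM-possessed characters are removed.
; Player list updates forward to the game state after a short delay.
; Initiative results go to the DM screen widget, reached through the screen actor's widget component.
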(event `self.K2_PostLogin`
  (params (NewPlayer :type "PlayerController Object Reference"))
  (bind _returnvalue (`|SpawnActorFromClass` "/Game/TTRPG/Character/Character_Default.Character_Default_C" (`KismetMathLibrary.MakeTransform` (0.0 0.0 0.0)) "Undefined" "MultiplyWithRoot" NewPlayer null))
  (`Controller.Possess` NewPlayer _returnvalue)
  (`KismetArrayLibrary.Array_Add` (`self.AllPlayerPawns`) _returnvalue))

(event `UpdatePlayerList`
  (`KismetSystemLibrary.Delay` 0.3)
  (bind _asbp_ttrpgvr_game_state (cast `/Game/TTRPG/GameMode/BP_TTRPGVR_GameState` (`GameplayStatics.GetGameState`)))
  (`/Game/TTRPG/GameMode/BP_TTRPGVR_GameState.UpdatePlayerList` _asbp_ttrpgvr_game_state))

(event `DMPossessed`
  (params (InCharacter :type "/Game/TTRPG/Character/Character_Default Object Reference"))
  (`KismetArrayLibrary.Array_RemoveItem` (`self.AllPlayerPawns`) InCharacter))

(event `self.K2_OnLogout`
  (params (ExitingController :type "Controller Object Reference")))

(event `AddInitiativeResult`
  (params (CharacterName :type Text) (InitiativeResult :type Text))
  (bind _returnvalue (`GameplayStatics.GetActorOfClass` "/Game/TTRPG/UI/Actor/UI_DMScreenActor.UI_DMScreenActor_C"))
  (bind _aswbp_dmscreen (cast `/Game/TTRPG/UI/WBP_DMScreen` (`WidgetComponent.GetWidget` (`/Game/TTRPG/UI/Actor/UI_DMScreenActor.Widget` _returnvalue))))
  (`/Game/TTRPG/UI/WBP_DMScreen.AddInitiativeResult` _aswbp_dmscreen CharacterName InitiativeResult))

(fn `UserConstructionScript`)